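; Fighter in an automatic turn-based duel that trades hits with its Enemy and shows health and item icons on the Battle_Hud widget by player Id.
; On BeginPlay it spawns an item per type and adds their stats to its own.
; Tick runs a ChangeTurn macro using initiative, IsAttacked flags and a delay to time attacks.
; Hits can crit for double damage and are reduced by armor; Die's body is unwired.
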(event `self.ReceiveBeginPlay`
  (`self.GetWidget`)
  (`self.SetItems`)
  (`self.UpdateWidget`))

(event `self.ReceiveTick`
  (params (DeltaSeconds :type "Float (single-precision)"))
  (if (not (`self.IsDead`))
    (`self.ChangeTurn`
      (:`NewParam2`
        (bind _dmg (`self.GetResultDmg` 0))
        (`self.TakeDmg` (`self.Enemy`) _dmg)))))

(fn `Die`)

(fn `GetPercentHp`
  (returns (Percent :type "Float (double-precision)"))
  (locals (Koef :type "Float (double-precision)"))
  (bind (_data_arm _data_hp) (break `/Game/BP/Char_BP/Char_Data` (`self.Data`)))
  (bind _output_get (set `local.Koef` (/ (`KismetMathLibrary.Conv_IntToDouble` (`self.MaxHp`)) 100.0)))
  (return (/ (/ (`KismetMathLibrary.Conv_IntToDouble` _data_hp) _output_get) 100.0)))

(fn `GetResultDmg`
  (params (BonusDmg :type Integer))
  (returns (Dmg :type Integer))
  (locals (ResDmg :type Integer))
  (bind (_data_arm _data_hp _data_dmg) (break `/Game/BP/Char_BP/Char_Data` (`self.Data`)))
  (bind _returnvalue (+ BonusDmg _data_dmg))
  (bind _iscreate (`self.IsCrit`))
  (if _iscreate
    (set `local.ResDmg` (* _returnvalue 2))
    (else
      (set `local.ResDmg` _returnvalue)))
  (return (`local.ResDmg`)))

(fn `GetWidget`
  (bind _asbattle_hud (cast `/Game/BP/Battle_Hud` (`PlayerController.GetHUD` (`GameplayStatics.GetPlayerController` 0)))
    (:`then`
      (set `self.Widget` (`/Game/BP/Battle_Hud.Widget` _asbattle_hud))
      (`KismetSystemLibrary.PrintString` "Succcesd"))
    (:`CastFailed`
      (`KismetSystemLibrary.PrintString` "FAileeeeeeed"))))

(fn `IsCrit`
  (returns (IsCreate :type Boolean))
  (bind (_data_arm _data_hp _data_dmg _data_critchance) (break `/Game/BP/Char_BP/Char_Data` (`self.Data`)))
  (return (>= _data_critchance (`KismetMathLibrary.RandomIntegerFromStream` 101 (`KismetMathLibrary.MakeRandomStream` (`GameplayStatics.GetAccurateRealTime`))))))

(fn `IsDie`
  (params (Dmg :type Integer))
  (bind (_data_arm _data_hp) (break `/Game/BP/Char_BP/Char_Data` (`self.Data`)))
  (`self.UpdateHp` (* Dmg -1))
  (`self.UpdateWidgetHP`)
  (`self.UpdateWigetItem`)
  (if (<= _data_hp 0)
    (set `self.IsDead` true)
    (`self.Die`)
    (return)))

(fn `IsFirstTurn`
  (returns (Is :type Boolean))
  (bind (_data_arm _data_hp _data_dmg _data_critchance _data_initiative) (break `/Game/BP/Char_BP/Char_Data` (`self.Data`)))
  (bind (_data_arm_2 _data_hp_2 _data_dmg_2 _data_critchance_2 _data_initiative_2) (break `/Game/BP/Char_BP/Char_Data` (`/Game/BP/Char_BP/BP_Player.Data` (`self.Enemy`))))
  (bind _output_get (set `self.IsAttacked` (not (> _data_initiative _data_initiative_2))))
  (set `/Game/BP/Char_BP/BP_Player.IsAttacked` (not _output_get) (`self.Enemy`))
  (return false))

(fn `SetItems`
  (bind _returnvalue (`self.GetTransform`))
  (bind _enumvalue (foreach `/Game/BP/Item_BP/Item_Types`)
    (:`LoopBody`
      (if (not (`|EnumEquality` _enumvalue "NewEnumerator5"))
        (bind _returnvalue_2 (`|SpawnActorFromClass` (`BlueprintMapLibrary.Map_Find` (`self.Items`) _enumvalue) (`KismetMathLibrary.MakeTransform` (`KismetMathLibrary.MakeVector` (.x (.location _returnvalue)) (.y (.location _returnvalue)) (+ (.z (.location _returnvalue)) 400.0)) (.rotation _returnvalue) (.scale _returnvalue)) "Undefined" "OverrideRootScale" self))
        (bind _data (`/Game/BP/Item_BP/Item.Data` _returnvalue_2))
        (`BlueprintMapLibrary.Map_Add` (`self.SpawnItems`) (break `/Game/BP/Item_BP/Item_Data` _data) _returnvalue_2)
        (`self.UpdateData` (break `/Game/BP/Char_BP/Char_Data` (`.Stats_15_0F93F9ED4750B1820DB122B5B77143B5` (break `/Game/BP/Item_BP/Item_Data` _data))) (`.Hp_9_FDBD932B4C0D27B1DCC76DBD6C40B8BC` (break `/Game/BP/Char_BP/Char_Data` (`.Stats_15_0F93F9ED4750B1820DB122B5B77143B5` (break `/Game/BP/Item_BP/Item_Data` _data)))) (`.Dmg_6_27FB3FA549389CD75EF40AA56ECEA0D8` (break `/Game/BP/Char_BP/Char_Data` (`.Stats_15_0F93F9ED4750B1820DB122B5B77143B5` (break `/Game/BP/Item_BP/Item_Data` _data)))) (`.CritChance_11_7EF125B54F5152004A93C69672EF9B77` (break `/Game/BP/Char_BP/Char_Data` (`.Stats_15_0F93F9ED4750B1820DB122B5B77143B5` (break `/Game/BP/Item_BP/Item_Data` _data)))) (`.Initiative_14_6EB32CBD4A50740F3F9B68B8AC90562D` (break `/Game/BP/Char_BP/Char_Data` (`.Stats_15_0F93F9ED4750B1820DB122B5B77143B5` (break `/Game/BP/Item_BP/Item_Data` _data)))))))))

(fn `TakeDmg`
  (params (Dmg :type Integer))
  (locals (dmg_taken :type Integer))
  (bind _data_arm (break `/Game/BP/Char_BP/Char_Data` (`self.Data`)))
  (bind _output_get (set `local.dmg_taken` Dmg))
  (set `local.dmg_taken` (- _output_get _data_arm))
  (`GameplayStatics.PlaySound2D` "/Game/Sound/hitOld00.hitOld00")
  (`self.IsDie` (`local.dmg_taken`))
  (`KismetSystemLibrary.PrintString` "HIT!"))

(fn `UpdateArm`
  (params (Arm :type Integer))
  (bind (_data_arm _data_hp _data_dmg) (break `/Game/BP/Char_BP/Char_Data` (`self.Data`)))
  (set `self.Data` (make `/Game/BP/Char_BP/Char_Data` (+ Arm _data_arm) 0 _data_dmg)))

(fn `UpdateData`
  (params (Arm :type Integer :default 0) (Hp :type Integer :default 0) (Dmg :type Integer :default 0) (CritChance :type Integer :default 0) (Initiative :type Integer :default 0))
  (bind (_data_arm _data_hp _data_dmg _data_critchance _data_initiative) (break `/Game/BP/Char_BP/Char_Data` (`self.Data`)))
  (bind _returnvalue (+ Hp _data_hp))
  (set `self.Data` (make `/Game/BP/Char_BP/Char_Data` (+ Arm _data_arm) _returnvalue (+ Dmg _data_dmg) (+ _data_critchance CritChance) (+ _data_initiative Initiative)))
  (set `self.MaxHp` _returnvalue))

(fn `UpdateDmg`
  (params (Dmg :type Integer))
  (bind (_data_arm _data_hp _data_dmg) (break `/Game/BP/Char_BP/Char_Data` (`self.Data`)))
  (set `self.Data` (make `/Game/BP/Char_BP/Char_Data` 0 0 (+ Dmg _data_dmg))))

(fn `UpdateHp`
  (params (Hp :type Integer))
  (bind (_data_arm _data_hp _data_dmg) (break `/Game/BP/Char_BP/Char_Data` (`self.Data`)))
  (set `self.Data` (make `/Game/BP/Char_BP/Char_Data` 0 (+ Hp _data_hp) _data_dmg)))

(fn `UpdateStats`)

(fn `UpdateWidget`
  (`self.UpdateWidgetHP`)
  (`self.UpdateWigetItem`))

(fn `UpdateWidgetHP`
  (bind _widget (`self.Widget`))
  (bind (_data_arm _data_hp) (break `/Game/BP/Char_BP/Char_Data` (`self.Data`)))
  (bind (_data_arm_2 _data_hp_2) (break `/Game/BP/Char_BP/Char_Data` (`self.Data`)))
  (bind _widget_2 (`self.Widget`))
  (if (== (`self.id`) 1)
    (bind _percent (`self.GetPercentHp`))
    (`self.GetWidget`)
    (bind _output_get (set `/Game/BP/Char_BP/Battle_Widget.Health_Player1` _percent _widget))
    (set `/Game/BP/Char_BP/Battle_Widget.Hp1` (`KismetStringLibrary.Conv_IntToString` _data_hp) _widget)
    (`KismetSystemLibrary.PrintString` (`KismetStringLibrary.Concat_StrStr` (`KismetStringLibrary.Conv_DoubleToString` _output_get) " :1"))
    (else
      (bind _percent_2 (`self.GetPercentHp`))
      (`self.GetWidget`)
      (bind _output_get_2 (set `/Game/BP/Char_BP/Battle_Widget.Health_Player2` _percent_2 _widget_2))
      (set `/Game/BP/Char_BP/Battle_Widget.Hp2` (`KismetStringLibrary.Conv_IntToString` _data_hp_2) _widget_2)
      (`KismetSystemLibrary.PrintString` (`KismetStringLibrary.Concat_StrStr` (`KismetStringLibrary.Conv_DoubleToString` _output_get_2) " :2")))))

(fn `UpdateWigetItem`
  (locals (Icon :type "Array of SlateBrush Structure") (E :type "/Game/BP/Item_BP/Item_Types Enum"))
  (bind _icon (`local.Icon`))
  (bind (_data_type _data_stats _data_icon) (break `/Game/BP/Item_BP/Item_Data` (`/Game/BP/Item_BP/Item.Data` (`BlueprintMapLibrary.Map_Find` (`self.SpawnItems`) (`local.E`)))))
  (bind _enumvalue (foreach `/Game/BP/Item_BP/Item_Types`)
    (:`LoopBody`
      (if (not (`|EnumEquality` _enumvalue "NewEnumerator5"))
        (set `local.E` _enumvalue)
        (`KismetArrayLibrary.Array_Add` (`local.Icon`) (make `SlateBrush` (`KismetMathLibrary.MakeVector2D` (`KismetMathLibrary.Conv_IntToDouble` (`Texture2D.Blueprint_GetSizeX` _data_icon)) (`KismetMathLibrary.Conv_IntToDouble` (`Texture2D.Blueprint_GetSizeY` _data_icon))) "Image" (struct) (struct :`SpecifiedColor` (struct :`R` 1.0 :`G` 1.0 :`B` 1.0 :`A` 1.0) :`ColorUseRule` "UseColor_Specified") "NoTile" "NoMirror" _data_icon))))
    (:`then`
      (if (== (`self.id`) 1)
        (set `/Game/BP/Char_BP/Battle_Widget.Icons_player_1` _icon (`self.Widget`))
        (else
          (set `/Game/BP/Char_BP/Battle_Widget.Icons_player_2` _icon (`self.Widget`)))))))

(fn `UserConstructionScript`)