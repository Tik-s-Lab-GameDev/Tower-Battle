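; BP_Player is a duelist in an automatic turn-based battle, trading hits with an Enemy reference until dead.
; Tick runs the ChangeTurn macro, which orders first turns by Initiative, then alternates IsAttacked flags after a one-second delay.
; Hits add bonus damage, can crit via a time-seeded roll, and lose Armor before reducing Hp.
; BeginPlay spawns owned item actors; damage updates the Id-selected HUD side, with item icons only for player one.
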(event `self.ReceiveBeginPlay`
  (set `self.Hp` (`self.MaxHp`))
  (`self.SetItems`))

(event `self.ReceiveTick`
  (params (DeltaSeconds :type "Float (single-precision)"))
  (if (not (`self.IsDead`))
    (`self.ChangeTurn`
      (:`NewParam2`
        (bind _dmg (`self.GetResultDmg` (`self.Bonus`)))
        (`self.TakeDmg` (`self.Enemy`) _dmg)))))

(event `Key|K`
  (params (Key :type "Key Structure" :default "AnyKey"))
  (:`Pressed`
    (bind _isa (`/Engine/EditorBlueprintResources/StandardMacros.FlipFlop`)
      (:`A`
        _)
      (:`B`
        _))
    (set `self.IsStart` _isa)
    (`KismetSystemLibrary.PrintString` "Hello")))

(fn `Die`
  (set `self.Hp` 0)
  (`self.UpdateWidget`)
  (`GameplayStatics.PlaySound2D` "/Game/Sound/gong1.gong1")
  (`KismetSystemLibrary.PrintString` "DEAD!!"))

(fn `GetPercentHp`
  (returns (Percent :type "Float (double-precision)"))
  (locals (Koef :type "Float (double-precision)"))
  (bind _output_get (set `local.Koef` (/ (`KismetMathLibrary.Conv_IntToDouble` (`self.MaxHp`)) 100.0)))
  (return (/ (/ (`KismetMathLibrary.Conv_IntToDouble` (`self.Hp`)) _output_get) 100.0)))

(fn `GetResultDmg`
  (params (BonusDmg :type Integer))
  (returns (Dmg :type Integer))
  (locals (ResDmg :type Integer))
  (bind _returnvalue (+ BonusDmg (`self.Dmg`)))
  (bind _iscreate (`self.IsCrit`))
  (if _iscreate
    (set `local.ResDmg` (* _returnvalue 2))
    (else
      (set `local.ResDmg` _returnvalue)))
  (return (`local.ResDmg`)))

(fn `GetWidget`
  (bind _asbattle_hud (cast `/Game/BP/Battle_Hud` (`PlayerController.GetHUD` (`GameplayStatics.GetPlayerController` 0))))
  (set `self.Widget` (`/Game/BP/Battle_Hud.Widget` _asbattle_hud)))

(fn `IsCrit`
  (returns (IsCreate :type Boolean))
  (return (>= (`self.CritChance`) (`KismetMathLibrary.RandomIntegerFromStream` 101 (`KismetMathLibrary.MakeRandomStream` (`GameplayStatics.GetAccurateRealTime`))))))

(fn `IsDie`
  (params (Dmg :type Integer))
  (set `self.Hp` (- (`self.Hp`) Dmg))
  (`self.UpdateWidget`)
  (if (<= (`self.Hp`) 0)
    (set `self.IsDead` true)
    (`self.Die`)
    (return)))

(fn `IsFirstTurn`
  (returns (Is :type Boolean))
  (bind _output_get (set `self.IsAttacked` (> (`self.Initiative`) (`/Game/BP/BP_Player.Initiative` (`self.Enemy`)))))
  (set `/Game/BP/BP_Player.IsAttacked` (not _output_get) (`self.Enemy`))
  (return false))

(fn `SetItems`
  (for _array_element (`self.Items`)
    (bind _returnvalue (`|SpawnActorFromClass` _array_element (`self.GetTransform`) "Undefined" "OverrideRootScale"))
    (set `/Game/BP/Item.OwnerPlayer` self _returnvalue)
    (`KismetArrayLibrary.Array_Add` (`self.SpawnItems`) _returnvalue)
    (`/Game/BP/Item.WasSpawned` _returnvalue)))

(fn `TakeDmg`
  (params (Dmg :type Integer))
  (locals (dmg_taken :type Integer))
  (bind _output_get (set `local.dmg_taken` Dmg))
  (set `local.dmg_taken` (- _output_get (`self.Armor`)))
  (`GameplayStatics.PlaySound2D` "/Game/Sound/hitOld00.hitOld00")
  (`self.IsDie` (`local.dmg_taken`))
  (`KismetSystemLibrary.PrintString` "HIT!"))

(fn `UpdateItemIcon`
  (set `/Game/BP/Battle_Widget.Image1_1` (make `SlateBrush` (64.0 64.0) "Image" (struct) (struct :`SpecifiedColor` (struct :`R` 1.0 :`G` 1.0 :`B` 1.0 :`A` 1.0) :`ColorUseRule` "UseColor_Specified") "NoTile" "NoMirror" (`/Game/BP/Item.Icon` (`|GetArrayItem` (`self.SpawnItems`)))) (`self.Widget`))
  (set `/Game/BP/Battle_Widget.Image1_2` (make `SlateBrush` (64.0 64.0) "Image" (struct) (struct :`SpecifiedColor` (struct :`R` 1.0 :`G` 1.0 :`B` 1.0 :`A` 1.0) :`ColorUseRule` "UseColor_Specified") "NoTile" "NoMirror" (`/Game/BP/Item.Icon` (`|GetArrayItem` (`self.SpawnItems`) 1))) (`self.Widget`))
  (set `/Game/BP/Battle_Widget.Image1_3` (make `SlateBrush` (64.0 64.0) "Image" (struct) (struct :`SpecifiedColor` (struct :`R` 1.0 :`G` 1.0 :`B` 1.0 :`A` 1.0) :`ColorUseRule` "UseColor_Specified") "NoTile" "NoMirror" (`/Game/BP/Item.Icon` (`|GetArrayItem` (`self.SpawnItems`) 2))) (`self.Widget`))
  (set `/Game/BP/Battle_Widget.Image1_4` (make `SlateBrush` (64.0 64.0) "Image" (struct) (struct :`SpecifiedColor` (struct :`R` 1.0 :`G` 1.0 :`B` 1.0 :`A` 1.0) :`ColorUseRule` "UseColor_Specified") "NoTile" "NoMirror" (`/Game/BP/Item.Icon` (`|GetArrayItem` (`self.SpawnItems`) 3))) (`self.Widget`))
  (set `/Game/BP/Battle_Widget.Image1_5` (make `SlateBrush` (64.0 64.0) "Image" (struct) (struct :`SpecifiedColor` (struct :`R` 1.0 :`G` 1.0 :`B` 1.0 :`A` 1.0) :`ColorUseRule` "UseColor_Specified") "NoTile" "NoMirror" (`/Game/BP/Item.Icon` (`|GetArrayItem` (`self.SpawnItems`) 4))) (`self.Widget`)))

(fn `UpdateItemIcon2`)

(fn `UpdateWidget`
  (bind _widget (`self.Widget`))
  (bind _widget_2 (`self.Widget`))
  (`self.GetWidget`)
  (if (== (`self.id`) 1)
    (bind _percent (`self.GetPercentHp`))
    (set `/Game/BP/Battle_Widget.Health_Player1` _percent _widget)
    (set `/Game/BP/Battle_Widget.Hp1` (`KismetStringLibrary.Conv_IntToString` (`self.Hp`)) _widget)
    (`self.UpdateItemIcon`)
    (else
      (bind _percent_2 (`self.GetPercentHp`))
      (set `/Game/BP/Battle_Widget.Health_Player2` _percent_2 _widget_2)
      (set `/Game/BP/Battle_Widget.Hp2` (`KismetStringLibrary.Conv_IntToString` (`self.Hp`)) _widget_2)
      (`self.UpdateItemIcon2`))))

(fn `UserConstructionScript`)